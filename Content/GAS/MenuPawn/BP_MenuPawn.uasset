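; BP_MenuPawn is the pawn for the main menu, setting up menu input, UI and music.
; On BeginPlay it replaces the player controller's Enhanced Input mappings with IMC_Menu, then creates WBP_MainMenu and adds it to the viewport.
; A second sequence branch plays the menu music as 2D sound.
; Tick is empty, and a camera yaw rotation is left unconnected, so it never runs.
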(event EventBeginPlay
  (Utilities|FlowControl|Sequence
    (:then_0
      (bind _asplayer_controller (Utilities|Casting|CastToPlayerController (Pawn|GetController)))
      (Class|EnhancedInputSubsystemInterface|ClearAllMappings (PlayerController|LocalPlayerSubsystems|GetEnhancedInputLocalPlayerSubsystem _asplayer_controller))
      (Input|AddMappingContext (PlayerController|LocalPlayerSubsystems|GetEnhancedInputLocalPlayerSubsystem _asplayer_controller) "/Game/GAS/MenuPawn/Inputs/Actions/IMC_Menu.IMC_Menu" 0 "(bIgnoreAllPressedKeysUntilRelease=True,bForceImmediately=False,bNotifyUserSettings=False)")
      (bind _returnvalue (UserInterface|CreateWidget "/Game/Menus/WBP_MainMenu.WBP_MainMenu_C" (Game|GetPlayerController 0)))
      (UserInterface|Viewport|AddtoViewport _returnvalue 0))
    (:then_1
      (Audio|PlaySound2D "/Game/Free_Fantasy_Music_Pack/Wav/Menu_Themes/MS_Menumusic.MS_Menumusic" 1.0 1.0 0.0 0 0))))

(event Collision|EventActorBeginOverlap
  (params (OtherActor :type Actor%20Object%20Reference)))

(event EventTick
  (params (DeltaSeconds :type Float%20%28single-precision%29)))

(fn ConstructionScript)